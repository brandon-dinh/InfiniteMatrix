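; BP_Projectile is a short-lived projectile that travels along world X and destroys itself on overlapping any actor other than BP_Player.
; On BeginPlay it sets its speed to twice the player's ForwardSpeed, then destroys itself after a two-second delay.
; Tick moves it with a swept, frame-rate-independent world offset, without a movement component.
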(event EventBeginPlay
  (bind _asbp_player (Utilities|Casting|CastToBP_Player (Game|Player|GetPlayerPawn 0)))
  (Variables|Default|SetProjectileSpeed (* (Variables|/Game/InfiniteMatrix/Blueprints/BP_Player.BP_Player_C|GetForwardSpeed _asbp_player) 2.0))
  (Utilities|FlowControl|Delay 2.0)
  (Actor|DestroyActor))

(event Collision|EventActorBeginOverlap
  (params (OtherActor :type Actor%20Object%20Reference))
  (Utilities|Casting|CastToBP_Player OtherActor
    (:CastFailed
      (Actor|DestroyActor))))

(event EventTick
  (params (DeltaSeconds :type Float%20%28single-precision%29))
  (Transformation|AddActorWorldOffset (Math|Vector|MakeVector (* DeltaSeconds (Variables|Default|GetProjectileSpeed)) 0.0 0.0) true))

(fn ConstructionScript)