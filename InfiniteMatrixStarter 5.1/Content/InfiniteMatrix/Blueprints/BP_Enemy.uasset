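; BP_Enemy is a short-lived enemy actor that destroys itself three seconds after BeginPlay.
; Overlapping BP_Player costs the player 10 health; at zero or below it flags the player dead, shows the restart display and destroys itself.
; Overlapping a BP_Projectile adds one to the score on player 0's pawn and destroys the enemy.
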(event EventBeginPlay
  (Utilities|FlowControl|Delay 3.0)
  (Actor|DestroyActor))

(event Collision|EventActorBeginOverlap
  (params (OtherActor :type Actor%20Object%20Reference))
  (bind _asbp_player (Utilities|Casting|CastToBP_Player OtherActor)
    (:then
      (bind _output_get (Variables|/Game/InfiniteMatrix/Blueprints/BP_Player.BP_Player_C|SetHealth _asbp_player (- (Variables|/Game/InfiniteMatrix/Blueprints/BP_Player.BP_Player_C|GetHealth _asbp_player) 1e+01)))
      (if (<= _output_get 0.0)
        (Variables|/Game/InfiniteMatrix/Blueprints/BP_Player.BP_Player_C|SetIsDead _asbp_player true)
        (Default|DisplayRestart _asbp_player)
        (Actor|DestroyActor)))
    (:CastFailed
      (Utilities|Casting|CastToBP_Projectile OtherActor)
      (bind _asbp_player_2 (Utilities|Casting|CastToBP_Player (Game|Player|GetPlayerPawn 0)))
      (Variables|/Game/InfiniteMatrix/Blueprints/BP_Player.BP_Player_C|SetScore _asbp_player_2 (+ (Variables|/Game/InfiniteMatrix/Blueprints/BP_Player.BP_Player_C|GetScore _asbp_player_2) 1))
      (Actor|DestroyActor))))

(event EventTick
  (params (DeltaSeconds :type Float%20%28single-precision%29)))

(fn ConstructionScript)